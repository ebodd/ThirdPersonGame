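; A sliding door that opens with the action button when the player holds its matching key.
; Overlapping the collision with the ThirdPersonCharacter enables player input on the door; leaving disables it and reverses the door.
; On press, it scans the character's Keys boolean array for a true entry at the door's KeyValue index, then plays the Open timeline to slide the Door's relative location.
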(event OnComponentBeginOverlap(Collision)
  (params (OverlappedComponent :type Primitive%20Component%20Object%20Reference) (OtherActor :type Actor%20Object%20Reference) (OtherComp :type Primitive%20Component%20Object%20Reference) (OtherBodyIndex :type Integer) (bFromSweep :type Boolean) (SweepResult :type Hit%20Result%20Structure%20%28by%20ref%29))
  (bind _asthird_person_character (Utilities|Casting|CastToThirdPersonCharacter OtherActor))
  (Input|EnableInput (Game|GetPlayerController 0)))

(event OnComponentEndOverlap(Collision)
  (params (OverlappedComponent :type Primitive%20Component%20Object%20Reference) (OtherActor :type Actor%20Object%20Reference) (OtherComp :type Primitive%20Component%20Object%20Reference) (OtherBodyIndex :type Integer))
  (Utilities|Casting|CastToThirdPersonCharacter OtherActor)
  (Input|DisableInput (Game|GetPlayerController 0))
  (bind _slide (Timeline|Open Reverse)
    (:Update
      (Transformation|SetRelativeLocation (Variables|Default|GetDoor) _slide false false))))

(event Input|ActionEvents|InputActionActionButton
  (params (Key :type Key%20Structure))
  (:Pressed
    (for (_array_element _array_index) (Variables|/Game/ThirdPersonCPP/Blueprints/ThirdPersonCharacter.ThirdPersonCharacter_C|GetKeys (stale OnComponentBeginOverlap(Collision) _asthird_person_character))
      (if (and _array_element (== _array_index (Variables|Default|GetKeyValue)))
        (bind _slide (Timeline|Open Play)
          (:Update
            (Transformation|SetRelativeLocation (Variables|Default|GetDoor) _slide false false)))))))

(fn ConstructionScript)